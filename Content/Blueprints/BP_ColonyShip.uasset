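; Colony ship actor that flies its flipbook sprite to an end location when launched, registered with the game mode for the win condition.
; On BeginPlay it stores itself in BP_GameMode and scales the launch timeline's play rate from a travel time in seconds.
; Launch events play the timeline, lerping the sprite's relative location.
; The construction script can preview the end location through a test flag, which is cleared at BeginPlay.
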(event Custom|PlayColonyLaunchFromStart
  ;[1 0.2812 0] Ship launch timeline
  (bind _lerp_alpha (Timeline|ColonyShipLaunchTimeline PlayFromStart)
    (:Update
      (Transformation|SetRelativeLocation (Variables|Default|GetPaperFlipbook) (Math|Vector|Lerp(Vector) "0,100.000000, 0" (Variables|PatrolInfo|GetEndLocation) _lerp_alpha) false false))))

(event Custom|PlayColonyLaunch
  ;[1 0.2812 0] Ship launch timeline
  (bind _lerp_alpha (Timeline|ColonyShipLaunchTimeline Play)
    (:Update
      (Transformation|SetRelativeLocation (Variables|Default|GetPaperFlipbook) (Math|Vector|Lerp(Vector) "0,100.000000, 0" (Variables|PatrolInfo|GetEndLocation) _lerp_alpha) false false))))

(event EventBeginPlay
  (|CallParentFunction)
  ;[0.1953 0 1] Set colony ship ref so win condition can be
  ; called later and play launch timeline
  (bind _asbp_game_mode (Utilities|Casting|CastToBP_GameMode (Game|GetGameMode)))
  (Variables|/Game/Blueprints/Game/BP_GameMode.BP_GameMode_C|SetColonyShipRef _asbp_game_mode self)
  (Components|Timeline|SetPlayRate (Variables|Default|GetColonyShipLaunchTimeline) (/ 1.0 (Variables|PatrolInfo|GetTravelTimeInSecconds)))
  (Variables|PatrolInfo|SetTestEndLocation? false))

(event Collision|EventActorBeginOverlap
  (params (OtherActor :type Actor%20Object%20Reference))
  (|CallParentFunction OtherActor) ; This node is disabled and will not be called.\nDrag off pins to build functionality.
)

(event EventTick
  (params (DeltaSeconds :type Float%20%28single-precision%29))
  (|CallParentFunction DeltaSeconds))

(fn ConstructionScript
  (|CallParentFunction)
  ;[0 1 0.1562] Test End Location
  (Transformation|SetRelativeLocation (Variables|Default|GetPaperFlipbook) (Math|Vector|SelectVector (Variables|PatrolInfo|GetEndLocation) "0,100.000000, 0" (Variables|PatrolInfo|GetTestEndLocation?)) false false))