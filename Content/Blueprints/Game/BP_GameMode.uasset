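; Game mode for a ship game that runs the countdown, fuel drain, music, main menu creation and win sequence.
; Tick uses delays to step the timer, dimming the sun and sounding alarms near expiry, and to drain fuel away from stations.
; Expired time or empty fuel kills the player, the latter guarded by a resettable DoOnce.
; Winning parks enemy ships, hides the player behind the map and launches the colony ship.
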(event Custom|ResetOutOfFuelDeath
  ;[1 0 0.6562] TICK - Countdown Timer, et al
  (Utilities|FlowControl|DoOnce false) ; enters at Reset
)

(event Custom|InitializeMainMenu
  ;[0.007812 1 0] Init Main Menu - Called from UI_GameTitleCredit
  (bind _asbp_game_mode (Utilities|Casting|CastToBP_GameMode (Game|GetGameMode)))
  (bind _returnvalue (UserInterface|CreateWidget "/Game/Blueprints/UI/UI_MainMenu.UI_MainMenu_C"))
  (Variables|BP_GameMode_C|SetMainMenuWidgetRef _asbp_game_mode _returnvalue)
  (UserInterface|Viewport|AddtoViewport _returnvalue 0))

(event Custom|ForTheWin
  ;[0 0.01562 1] Winner!
  (Utilities|HandlePlayerWin))

(event Custom|PlayGameMusic
  ;[0 0.7656 1] Play random game music - This is called from UI_GameTitleCredit, within the FadeIn Animation
  (Default|PlaySound (Variables|Default|GetGameMusicRef) (Utilities|Array|Get(acopy) (Variables|GameInfo|GetGameMusic) (Math|Random|RandomIntegerinRange 0 1)) 0.4))

(event EventBeginPlay
  ;[0.8047 1 0] Begin Play
  (CallFunction|ReferenceCasts)
  (Variables|Default|SetGameMusicRef (Variables|Default|GetBPC_Sounds)) ; Set ref so music can be \nstopped/started
  (Input|SetInputModeGameOnly (Variables|References|GetPlayerControllerRef))
  (CallFunction|InitializeEnemies))

(event EventTick
  (params (DeltaSeconds :type Float%20%28single-precision%29))
  (bind _playercontrollerref (Variables|References|GetPlayerControllerRef))
  ;[1 0 0.6562] TICK - Countdown Timer, et al
  (Utilities|IsValid _playercontrollerref
    (:Is%20Valid
      (if (not (Variables|/Game/Blueprints/Player/BP_PlayerController.BP_PlayerController_C|GetPaused? _playercontrollerref)) ; Don't tick if paused
        (if (Variables|GameInfo|GetStartGameTimer?) ; Don't tick if game not\nstarted
          (Utilities|FlowControl|Sequence
            (:then_0
              (Utilities|FlowControl|Delay (Variables|GameModifiers|GetCountdownSpeed)) ; Set to 1 to represent 1 second
              (CallFunction|ProcCountdownTimer))
            (:then_1
              (if (not (Variables|GameInfo|GetOnStation?)) ; Player at the station?\nIf so, don't use fuel
                (Utilities|FlowControl|Delay (Variables|GameModifiers|GetFuelDrainSpeed))
                (Utilities|ProcFuelCountdown
                  (:OutOfFuel
                    (Utilities|FlowControl|DoOnce false ; Only handle death once when fuel is empty
                      (:Completed
                        (CallFunction|OutOfFuelDeath)))))))))))))

(fn ConstructionScript)

(fn ReferenceCasts
  (bind _asbp_player_controller (Utilities|Casting|CastToBP_PlayerController (Game|GetPlayerController 0)))
  (Variables|References|SetPlayerControllerRef _asbp_player_controller)
  (bind _asbp_character (Utilities|Casting|CastToBP_Character (Game|GetPlayerCharacter 0)))
  (Variables|References|SetPlayerCharRef _asbp_character))

(fn DimtheSun
  ;[0.5937 1 0] Dim the Sun in the closing minutes of the game
  (if (not (< (Variables|GameModifiers|GetMinutesRemaining) 0)) ; Not Final minute of play?
    (switch int (Variables|GameModifiers|GetMinutesRemaining) ; Dim the Sun incrementally\nin last 4 minutes
      (:0
        (Variables|GameInfo|SetNewSunColor "(R=0.200000,G=0.200000,B=0.000000,A=1.000000)"))
      (:1
        (Variables|GameInfo|SetNewSunColor "(R=0.400000,G=0.400000,B=0.000000,A=1.000000)"))
      (:2
        (Variables|GameInfo|SetNewSunColor "(R=0.600000,G=0.600000,B=0.000000,A=1.000000)"))
      (:3
        (Variables|GameInfo|SetNewSunColor "(R=0.800000,G=0.800000,B=0.000000,A=1.000000)")))
    (Sprite|SetSpriteColor (Variables|/Game/Blueprints/BP_Sun.BP_Sun_C|GetPaperSprite (Variables|References|GetSunRef)) (Variables|GameInfo|GetNewSunColor))
    (else
      (Variables|GameInfo|SetNewSunColor "(R=0.000000,G=0.000000,B=0.000000,A=1.000000)")
      (Sprite|SetSpriteColor (Variables|/Game/Blueprints/BP_Sun.BP_Sun_C|GetPaperSprite (Variables|References|GetSunRef)) (Variables|GameInfo|GetNewSunColor)))))

(fn ProcCountdownTimer
  (bind _playercontrollerref (Variables|References|GetPlayerControllerRef))
  (if (not (Variables|GameInfo|GetGameOver?))
    (Variables|GameModifiers|SetSecondsRemaining (- (Variables|GameModifiers|GetSecondsRemaining) 1))
    (if (< (Variables|GameModifiers|GetSecondsRemaining) 0) ; Seconds < 0?
      (Variables|GameModifiers|SetMinutesRemaining (- (Variables|GameModifiers|GetMinutesRemaining) 1)) ; Remove 1 minute
      (if (Variables|GameInfo|GetFirstMinute?)
        (Variables|GameInfo|SetFirstMinute? false)
        (else
          (Default|PlaySound (Variables|Default|GetBPC_Sounds) "/Game/Sounds/TimerAlarm_Cue.TimerAlarm_Cue" 1.0) ; Warning on the minute
        ))
      (CallFunction|DimtheSun)
      (Variables|GameModifiers|SetSecondsRemaining 59) ; Reset Seconds to 59
      (if (<= (Variables|GameModifiers|GetMinutesRemaining) -1) ; Time expired?
        (Variables|GameInfo|SetStartGameTimer? false)
        (Variables|GameModifiers|SetSecondsRemaining 0)
        (Variables|GameModifiers|SetMinutesRemaining 0)
        ;[0 0.625 1] Game Over
        (Variables|/Game/Blueprints/Player/BP_PlayerController.BP_PlayerController_C|SetLivesRemaining _playercontrollerref 0)
        (Default|PlayerDeath _playercontrollerref)
        (Variables|GameInfo|SetFirstMinute? true))
      (elif (Math|Boolean|ANDBoolean (< (Variables|GameModifiers|GetSecondsRemaining) 10) (>= (Variables|GameModifiers|GetSecondsRemaining) 0) (== (Variables|GameModifiers|GetMinutesRemaining) 0)) ; Final 10 seconds in\ncountdown?
        (Default|PlaySound (Variables|Default|GetBPC_Sounds) "/Game/Sounds/TimerAlarm_Cue.TimerAlarm_Cue" 1.0) ; Last seconds audible\nwarning
      ))))

(fn InitializeEnemies
  (bind _outactors (Actor|GetAllActorsOfClass "/Game/Blueprints/Enemy/BP_EnemyShip.BP_EnemyShip_C"))
  (for _array_element _outactors
    (bind _asbp_enemy_ship (Utilities|Casting|CastToBP_EnemyShip _array_element))
    (Components|Timeline|PlayfromStart (Variables|/Game/Blueprints/Enemy/BP_EnemyShip.BP_EnemyShip_C|GetPatrolTimeline _asbp_enemy_ship)) ; sends enemy ships back to start
    (Audio|Components|Audio|Stop (Variables|/Game/Blueprints/Enemy/BP_EnemyShip.BP_EnemyShip_C|GetPatrolTimeline _asbp_enemy_ship)) ; Stops the timeline
  ))

(fn OutOfFuelDeath
  (Rendering|SetVisibility (Variables|/Game/Blueprints/Player/BP_Character.BP_Character_C|GetExplodeFlipbook (Variables|References|GetPlayerCharRef)) true true) ; Show explosion
  (Default|PlaySound (Variables|Default|GetBPC_Sounds) "/Game/Retro_8Bit_Sounds/Explosion/Wavs/retro_explosion_general_01.retro_explosion_general_01" 1.0)
  (Default|PlayerDeath (Variables|References|GetPlayerControllerRef)))