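; BPC_Patrol is a patrol component with functions for moving a given actor back and forth along the X axis.
; TravelForward and TravelBack set the actor's transform with opposite fixed yaws, both subtracting DistancePerTick from CurrentLocationX.
; Each compares CurrentLocationX to EndLocationX to set the Reverse flag.
; BeginPlay is empty, and nothing here calls either function or updates CurrentLocationX.
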(event EventBeginPlay)

(fn TravelForward
  (params (Actor :type Actor%20Object%20Reference) (NewTransform_Location_Y :type Float%20%28single-precision%29) (NewTransform_Location_Z :type Float%20%28single-precision%29))
  ;[0 0.6953 1] Travel Forward
  (Transformation|SetActorTransform Actor (Math|Transform|MakeTransform (Math|Vector|MakeVector (- (Variables|PatrolInfo|GetCurrentLocationX) (Variables|PatrolInfo|GetDistancePerTick)) NewTransform_Location_Y NewTransform_Location_Z) "270.000000, 0, 0" "1,1,1"))
  (if (== (Variables|PatrolInfo|GetCurrentLocationX) (Variables|PatrolInfo|GetEndLocationX)) ; Reached end of travel?
    (Variables|PatrolInfo|SetReverse? true)
    (else
      (Variables|PatrolInfo|SetReverse? false))))

(fn TravelBack
  (params (Actor :type Actor%20Object%20Reference) (NewTransform_Location_Y :type Float%20%28single-precision%29) (NewTransform_Location_Z :type Float%20%28single-precision%29))
  ;[0 0.6953 1] Travel Forward
  (Transformation|SetActorTransform Actor (Math|Transform|MakeTransform (Math|Vector|MakeVector (- (Variables|PatrolInfo|GetCurrentLocationX) (Variables|PatrolInfo|GetDistancePerTick)) NewTransform_Location_Y NewTransform_Location_Z) "90.000000, 0, 0" "1,1,1"))
  (if (== (Variables|PatrolInfo|GetCurrentLocationX) (Variables|PatrolInfo|GetEndLocationX)) ; Reached end of travel?
    (Variables|PatrolInfo|SetReverse? false)
    (else
      (Variables|PatrolInfo|SetReverse? true))))