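; Player controller for a 2D sprite ship game, handling movement, pause menu, HUD creation and the death/respawn cycle.
; The MovementControls macro turns axis input into swept pawn moves on local X/Z and snaps the sprite to face travel.
; Death spends a life and respawns at PlayerStart with full fuel, or shows game over through GameMode's menu, shared with RestartGame.
; Debug keys trigger win, fuel-out and countdown endings.
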(event Custom|PlayerDeath
  (bind _gamemoderef (Variables|References|GetGameModeRef))
  (bind _gamemoderef_2 (Variables|References|GetGameModeRef))
  (bind _controllerref (Variables|References|GetControllerRef))
  (bind _mainmenuwidgetref (Variables|/Game/Blueprints/Game/BP_GameMode.BP_GameMode_C|GetMainMenuWidgetRef _gamemoderef_2))
  ;[1 0.5156 0] Player Death
  (Utilities|FlowControl|Delay 2.0)
  (Variables|PlayerModifiers|SetDefaultPlayerMovementSpeed 5.0)
  (if (== (Variables|PlayerModifiers|GetLivesRemaining) 0) ; Out of lives?
    (Variables|/Game/Blueprints/Game/BP_GameMode.BP_GameMode_C|SetGameOver? (Variables|References|GetGameModeRef) true)
    (Rendering|Components|TextRender|SetText (Variables|/Game/Blueprints/UI/UI_MainMenu.UI_MainMenu_C|GetGameOutcomeMsgText (Variables|/Game/Blueprints/Game/BP_GameMode.BP_GameMode_C|GetMainMenuWidgetRef (Variables|References|GetGameModeRef))) "Sorry, you failed to save us.")
    (Game|SetGamePaused true)
    (CallFunction|RespawnPlayer)
    (UserInterface|Viewport|AddtoViewport _mainmenuwidgetref 0)
    (Input|SetInputModeUIOnly _controllerref 0 "DoNotLock")
    (Variables|/Script/Engine.PlayerController|SetbShowMouseCursor _controllerref true)
    (Rendering|Components|TextRender|SetText (Variables|/Game/Blueprints/UI/UI_MainMenu.UI_MainMenu_C|GetPlayBtnText _mainmenuwidgetref) "Play Again?")
    (else
      ;;[0 0.625 1] Update lives, empty cargo and respawn player
      (Variables|PlayerModifiers|SetLivesRemaining (- (Variables|PlayerModifiers|GetLivesRemaining) 1))
      (CallFunction|RespawnPlayer)
      (Variables|/Game/Blueprints/Player/BPC_PlayerShipInfo.BPC_PlayerShipInfo_C|SetCurrentCargoLoad (Variables|/Game/Blueprints/Player/BP_Character.BP_Character_C|GetBPC_PlayerShipInfo (Variables|References|GetPlayerCharRef)) 0.0)))
  (bind _outactors (Actor|GetAllActorsOfClass "/Game/Blueprints/Enemy/BP_EnemyShip.BP_EnemyShip_C"))
  (for _array_element _outactors
    (Default|PlayfromStart _array_element))
  (if (Variables|/Game/Blueprints/Game/BP_GameMode.BP_GameMode_C|GetGameOver? _gamemoderef)
    (Widget|SetVisibility (Variables|/Game/Blueprints/UI/UI_MainMenu.UI_MainMenu_C|GetGameOutcomeMsgText (Variables|/Game/Blueprints/Game/BP_GameMode.BP_GameMode_C|GetMainMenuWidgetRef _gamemoderef)) "Visible")))

(event Custom|RestartGame
  (bind _gamemoderef (Variables|References|GetGameModeRef))
  (bind _gamemoderef_2 (Variables|References|GetGameModeRef))
  (bind _controllerref (Variables|References|GetControllerRef))
  (bind _mainmenuwidgetref (Variables|/Game/Blueprints/Game/BP_GameMode.BP_GameMode_C|GetMainMenuWidgetRef _gamemoderef_2))
  ;[1 0.5156 0] Player Death
  (Variables|/Game/Blueprints/Game/BP_GameMode.BP_GameMode_C|SetCurrentColonyShipBuildStatus (Variables|References|GetGameModeRef) 0.0)
  (Game|SetGamePaused true)
  (CallFunction|RespawnPlayer)
  (UserInterface|Viewport|AddtoViewport _mainmenuwidgetref 0)
  (Input|SetInputModeUIOnly _controllerref 0 "DoNotLock")
  (Variables|/Script/Engine.PlayerController|SetbShowMouseCursor _controllerref true)
  (Rendering|Components|TextRender|SetText (Variables|/Game/Blueprints/UI/UI_MainMenu.UI_MainMenu_C|GetPlayBtnText _mainmenuwidgetref) "Play Again?")
  (bind _outactors (Actor|GetAllActorsOfClass "/Game/Blueprints/Enemy/BP_EnemyShip.BP_EnemyShip_C"))
  (for _array_element _outactors
    (Default|PlayfromStart _array_element))
  (if (Variables|/Game/Blueprints/Game/BP_GameMode.BP_GameMode_C|GetGameOver? _gamemoderef)
    (Widget|SetVisibility (Variables|/Game/Blueprints/UI/UI_MainMenu.UI_MainMenu_C|GetGameOutcomeMsgText (Variables|/Game/Blueprints/Game/BP_GameMode.BP_GameMode_C|GetMainMenuWidgetRef _gamemoderef)) "Visible")))

(event EventBeginPlay
  ;[0.05469 1 0] BeginPlay
  (CallFunction|ReferenceCasts)
  (bind _returnvalue (UserInterface|CreateWidget "/Game/Blueprints/UI/UI_HUD.UI_HUD_C")) ; Create player HUD
  (Variables|References|SetHUDRef _returnvalue)
  (UserInterface|Viewport|AddtoViewport _returnvalue 0)
  (Widget|SetVisibility _returnvalue "Hidden"))

(event Input|ActionEvents|InputActionPauseGame
  (params (Key :type Key%20Structure :default "None"))
  (bind _gamemoderef (Variables|References|GetGameModeRef))
  (bind _mainmenuwidgetref (Variables|/Game/Blueprints/Game/BP_GameMode.BP_GameMode_C|GetMainMenuWidgetRef _gamemoderef))
  ;[0.8984 1 0] Pause Game
  (:Pressed
    (Game|SetGamePaused true)
    (Variables|GameInfo|SetPaused? true)
    (Variables|Default|SetbShowMouseCursor true)
    (UserInterface|Viewport|AddtoViewport _mainmenuwidgetref 0)
    (Rendering|Components|TextRender|SetText (Variables|/Game/Blueprints/UI/UI_MainMenu.UI_MainMenu_C|GetPlayBtnText _mainmenuwidgetref) "Resume?")))

(event Input|AxisEvents|InputAxisMoveForward
  (params (AxisValue :type Float%20%28single-precision%29))
  ;[0 1 0.7188 0.5] Player Movement
  (Utilities|MovementControls AxisValue (stale Input|AxisEvents|InputAxisMoveRight AxisValue)))

(event Input|AxisEvents|InputAxisMoveRight
  (params (AxisValue :type Float%20%28single-precision%29))
  ;[0 1 0.7188 0.5] Player Movement
  (Utilities|MovementControls (stale Input|AxisEvents|InputAxisMoveForward AxisValue) AxisValue) ; enters at Right Movement
)

(event Input|KeyboardEvents|M
  (params (Key :type Key%20Structure :default "None"))
  ;[1 0 0.02836] Debug: M = Test Win condition
  (:Pressed
    (Default|FortheWin (Variables|References|GetGameModeRef))))

(event Input|KeyboardEvents|Escape
  (params (Key :type Key%20Structure :default "None"))
  (bind _gamemoderef (Variables|References|GetGameModeRef))
  (bind _mainmenuwidgetref (Variables|/Game/Blueprints/Game/BP_GameMode.BP_GameMode_C|GetMainMenuWidgetRef _gamemoderef))
  ;[0.8984 1 0] Pause Game
  (:Pressed
    (if (Variables|GameInfo|GetGameInProgress?)
      (Game|SetGamePaused true)
      (Variables|GameInfo|SetPaused? true)
      (Variables|Default|SetbShowMouseCursor true)
      (UserInterface|Viewport|AddtoViewport _mainmenuwidgetref 0)
      (Rendering|Components|TextRender|SetText (Variables|/Game/Blueprints/UI/UI_MainMenu.UI_MainMenu_C|GetPlayBtnText _mainmenuwidgetref) "Resume?"))))

(event Input|KeyboardEvents|F
  (params (Key :type Key%20Structure :default "None"))
  ;[1 0 0.2109] Debug: F = Test Fuel death
  (:Pressed
    (bind _asbp_character (Utilities|Casting|CastToBP_Character (Game|GetPlayerCharacter 0)))
    (Variables|/Game/Blueprints/BPC_Fuel.BPC_Fuel_C|SetCurrentFuel (Variables|/Game/Blueprints/Player/BP_Character.BP_Character_C|GetBPC_Fuel _asbp_character) 0.0)))

(event Input|KeyboardEvents|T
  (params (Key :type Key%20Structure :default "None"))
  (bind _gamemoderef (Variables|References|GetGameModeRef))
  ;[0 0.8828 1] Debug: T = Countdown ran out death
  (:Pressed
    (Variables|/Game/Blueprints/Game/BP_GameMode.BP_GameMode_C|SetMinutesRemaining _gamemoderef 0)
    (Variables|/Game/Blueprints/Game/BP_GameMode.BP_GameMode_C|SetSecondsRemaining _gamemoderef 5)))

(fn ConstructionScript)

(fn ReferenceCasts
  (bind _asbp_character (Utilities|Casting|CastToBP_Character (Game|Player|GetPlayerPawn 0)))
  (Variables|References|SetCameraPawnRef _asbp_character)
  (bind _asbp_game_mode (Utilities|Casting|CastToBP_GameMode (Game|GetGameMode)))
  (Variables|References|SetGameModeRef _asbp_game_mode)
  (bind _asbp_player_controller (Utilities|Casting|CastToBP_PlayerController (Game|GetPlayerController 0)))
  (Variables|References|SetControllerRef _asbp_player_controller))

(fn HandlePlayerDeath
  (CallFunction|PlayerDeath))

(fn RespawnPlayer
  (Default|ResetOutOfFuelDeath (Variables|References|GetGameModeRef))
  (bind _outactors (Actor|GetAllActorsOfClass "/Script/Engine.PlayerStart")) ; Find player start
  (bind _asbp_character (Utilities|Casting|CastToBP_Character (Game|GetPlayerCharacter 0)))
  (bind _output_get (Variables|References|SetPlayerCharRef _asbp_character))
  (Audio|PlaySound2D "/Game/Retro_8Bit_Sounds/Damage_Hurt/Wavs/retro_damage_hurt_ouch_11.retro_damage_hurt_ouch_11" 1.0 1.0 0.0 0 _output_get) ; Play respawn sound
  (Transformation|SetActorLocation _asbp_character (Transformation|GetActorLocation (Utilities|Array|Get(acopy) _outactors)) false false) ; Send back to player start
  (Rendering|SetVisibility (Variables|/Game/Blueprints/Player/BP_Character.BP_Character_C|GetExplodeFlipbook (Variables|References|GetPlayerCharRef)) false false) ; Hide player explosion
  (Variables|/Game/Blueprints/BPC_Fuel.BPC_Fuel_C|SetCurrentFuel (Variables|/Game/Blueprints/Player/BP_Character.BP_Character_C|GetBPC_Fuel (Variables|References|GetPlayerCharRef)) (Variables|/Game/Blueprints/BPC_Fuel.BPC_Fuel_C|GetMaxFuel (Variables|/Game/Blueprints/Player/BP_Character.BP_Character_C|GetBPC_Fuel (Variables|References|GetPlayerCharRef)))) ; Give player full fuel
)