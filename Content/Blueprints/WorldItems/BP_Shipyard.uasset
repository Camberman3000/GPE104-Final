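; BP_Shipyard is the station where the player delivers ore toward building the colony ship and refuels.
; Entering its box flags the player as on station and empties any cargo into the game mode's build total with a dumping sound.
; A delivery that would reach the maximum fills the total and triggers the win instead.
; While docked, Tick refills fuel to full through a short Delay; leaving the box clears the flag.
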(event OnComponentBeginOverlap(Box)
  (params (OverlappedComponent :type Primitive%20Component%20Object%20Reference) (OtherActor :type Actor%20Object%20Reference) (OtherComp :type Primitive%20Component%20Object%20Reference) (OtherBodyIndex :type Integer) (bFromSweep :type Boolean) (SweepResult :type Hit%20Result%20Structure%20%28by%20ref%29))
  ;[0 1 0.9531] Overlap shipyard - Empty Player ship
  (bind _asbp_character (Utilities|Casting|CastToBP_Character OtherActor))
  (Variables|References|SetPlayerCharRef _asbp_character)
  (Variables|/Game/Blueprints/Game/BP_GameMode.BP_GameMode_C|SetOnStation? (Variables|References|GetGameModeRef) true)
  (if (not (== (Variables|/Game/Blueprints/Player/BPC_PlayerShipInfo.BPC_PlayerShipInfo_C|GetCurrentCargoLoad (Variables|/Game/Blueprints/Player/BP_Character.BP_Character_C|GetBPC_PlayerShipInfo (Variables|References|GetPlayerCharRef))) 0.0)) ; Ship empty?
    (Utilities|CheckWinCondition
      (:Win
        (CallFunction|ProcessPlayerWin))
      (:No%20Win
        (CallFunction|CollectOrefromPlayerShip)))))

(event OnComponentEndOverlap(Box)
  (params (OverlappedComponent :type Primitive%20Component%20Object%20Reference) (OtherActor :type Actor%20Object%20Reference) (OtherComp :type Primitive%20Component%20Object%20Reference) (OtherBodyIndex :type Integer))
  ;[0.7109 1 0] End Overlap
  (Variables|/Game/Blueprints/Game/BP_GameMode.BP_GameMode_C|SetOnStation? (Variables|References|GetGameModeRef) false))

(event EventBeginPlay
  (bind _asbp_game_mode (Utilities|Casting|CastToBP_GameMode (Game|GetGameMode)))
  (Variables|References|SetGameModeRef _asbp_game_mode))

(event Collision|EventActorBeginOverlap
  (params (OtherActor :type Actor%20Object%20Reference)))

(event EventTick
  (params (DeltaSeconds :type Float%20%28single-precision%29))
  (if (Variables|/Game/Blueprints/Game/BP_GameMode.BP_GameMode_C|GetOnStation? (Variables|References|GetGameModeRef))
    (Utilities|FlowControl|Delay 0.2)
    (CallFunction|RefillFuel)))

(fn ConstructionScript)

(fn ProcessPlayerWin
  (bind _gamemoderef (Variables|References|GetGameModeRef))
  (Variables|/Game/Blueprints/Player/BPC_PlayerShipInfo.BPC_PlayerShipInfo_C|SetCurrentCargoLoad (Variables|/Game/Blueprints/Player/BP_Character.BP_Character_C|GetBPC_PlayerShipInfo (Variables|References|GetPlayerCharRef)) 0.0)
  (Variables|/Game/Blueprints/Game/BP_GameMode.BP_GameMode_C|SetCurrentColonyShipBuildStatus _gamemoderef (Variables|/Game/Blueprints/Game/BP_GameMode.BP_GameMode_C|GetMaxColonyShipBuildStatus _gamemoderef))
  (Default|FortheWin (Variables|References|GetGameModeRef)))

(fn CollectOrefromPlayerShip
  (bind _gamemoderef (Variables|References|GetGameModeRef))
  (Variables|/Game/Blueprints/Game/BP_GameMode.BP_GameMode_C|SetCurrentColonyShipBuildStatus _gamemoderef (+ (Variables|/Game/Blueprints/Game/BP_GameMode.BP_GameMode_C|GetCurrentColonyShipBuildStatus _gamemoderef) (Variables|/Game/Blueprints/Player/BPC_PlayerShipInfo.BPC_PlayerShipInfo_C|GetCurrentCargoLoad (Variables|/Game/Blueprints/Player/BP_Character.BP_Character_C|GetBPC_PlayerShipInfo (Variables|References|GetPlayerCharRef)))))
  (Variables|/Game/Blueprints/Player/BPC_PlayerShipInfo.BPC_PlayerShipInfo_C|SetCurrentCargoLoad (Variables|/Game/Blueprints/Player/BP_Character.BP_Character_C|GetBPC_PlayerShipInfo (Variables|References|GetPlayerCharRef)) 0.0)
  (Default|PlaySound (Variables|Default|GetBPC_Sounds) "/Game/Sounds/ShipDumpingSound_Cue.ShipDumpingSound_Cue" 1.0))

(fn RefillFuel
  (bind _playercharref (Variables|References|GetPlayerCharRef))
  (bind _bpc_fuel (Variables|/Game/Blueprints/Player/BP_Character.BP_Character_C|GetBPC_Fuel _playercharref))
  (Variables|/Game/Blueprints/BPC_Fuel.BPC_Fuel_C|SetCurrentFuel _bpc_fuel (Variables|/Game/Blueprints/BPC_Fuel.BPC_Fuel_C|GetMaxFuel _bpc_fuel)))