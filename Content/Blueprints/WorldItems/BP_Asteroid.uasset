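; Mineable, spinning 2D asteroid that adds ore to the player ship's cargo on overlap.
; Construction randomizes pitch and scale, and enlarges the collision sphere by a random amount.
; Overlap reports a full hold, or zeroes player speed, plays laser sound and brings the effect flipbook forward.
; After a two-second delay it shifts the asteroid sprite back in Y, restores speed and adds ore capped at capacity.
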(event OnComponentBeginOverlap(Sphere)
  (params (OverlappedComponent :type Primitive%20Component%20Object%20Reference) (OtherActor :type Actor%20Object%20Reference) (OtherComp :type Primitive%20Component%20Object%20Reference) (OtherBodyIndex :type Integer) (bFromSweep :type Boolean) (SweepResult :type Hit%20Result%20Structure%20%28by%20ref%29))
  (bind _paperflipbook (Variables|Default|GetPaperFlipbook))
  (bind _playercharref (Variables|Default|GetPlayerCharRef))
  (bind _playercontrollerref (Variables|Default|GetPlayerControllerRef))
  (bind _playercharref_2 (Variables|Default|GetPlayerCharRef))
  (bind _rendercomponent (Variables|Default|GetRenderComponent))
  (bind _returnvalue (Transformation|GetWorldLocation _rendercomponent))
  (bind _returnvalue_2 (Transformation|GetWorldLocation _paperflipbook))
  (bind _bpc_playershipinfo (Variables|/Game/Blueprints/Player/BP_Character.BP_Character_C|GetBPC_PlayerShipInfo _playercharref_2))
  (bind _bpc_playershipinfo_2 (Variables|/Game/Blueprints/Player/BP_Character.BP_Character_C|GetBPC_PlayerShipInfo _playercharref))
  (bind (_x _y _z) (Math|Vector|BreakVector _returnvalue_2))
  (bind _maxcargoload (Variables|/Game/Blueprints/Player/BPC_PlayerShipInfo.BPC_PlayerShipInfo_C|GetMaxCargoLoad _bpc_playershipinfo_2))
  ;[1 0.04688 0] Overlap
  (CallFunction|ReferenceCasts OtherActor)
  (Utilities|IsValid _playercharref_2
    (:Is%20Valid
      (if (== (Variables|/Game/Blueprints/Player/BPC_PlayerShipInfo.BPC_PlayerShipInfo_C|GetCurrentCargoLoad _bpc_playershipinfo) (Variables|/Game/Blueprints/Player/BPC_PlayerShipInfo.BPC_PlayerShipInfo_C|GetMaxCargoLoad _bpc_playershipinfo))
        (Development|PrintString "SHIP IS FULL")
        (else
          (Utilities|IsValid _playercontrollerref
            (:Is%20Valid
              (Variables|Default|SetOriginalPlayerMovementSpeed (Variables|/Game/Blueprints/Player/BP_PlayerController.BP_PlayerController_C|GetDefaultPlayerMovementSpeed _playercontrollerref))
              (Variables|/Game/Blueprints/Player/BP_PlayerController.BP_PlayerController_C|SetDefaultPlayerMovementSpeed _playercontrollerref 0.0)
              (Default|PlaySound (Variables|Default|GetBPC_Sounds) "/Game/Sounds/MiningLaserSound_Cue.MiningLaserSound_Cue" 1.0)
              (Transformation|SetWorldLocation _paperflipbook (Math|Vector|MakeVector _x (+ _y 4e+01) _z) false false) ; Bring mining effect flipbook to the front
              (Utilities|FlowControl|Delay 2.0)
              (Transformation|SetWorldLocation _rendercomponent (Math|Vector|MakeVector (.x _returnvalue) (- (.y _returnvalue) 1e+03) (.z _returnvalue)) false false) ; Send mining effect behind the asteroid (Hidden)
              (Variables|/Game/Blueprints/Player/BP_PlayerController.BP_PlayerController_C|SetDefaultPlayerMovementSpeed (Variables|Default|GetPlayerControllerRef) (Variables|Default|GetOriginalPlayerMovementSpeed))
              (if (>= (+ (Variables|/Game/Blueprints/Player/BPC_PlayerShipInfo.BPC_PlayerShipInfo_C|GetCurrentCargoLoad _bpc_playershipinfo_2) (Variables|AsteroidInfo|GetOre)) _maxcargoload)
                (Variables|/Game/Blueprints/Player/BPC_PlayerShipInfo.BPC_PlayerShipInfo_C|SetCurrentCargoLoad _bpc_playershipinfo_2 _maxcargoload)
                (else
                  (Variables|/Game/Blueprints/Player/BPC_PlayerShipInfo.BPC_PlayerShipInfo_C|SetCurrentCargoLoad _bpc_playershipinfo_2 (+ (Variables|/Game/Blueprints/Player/BPC_PlayerShipInfo.BPC_PlayerShipInfo_C|GetCurrentCargoLoad _bpc_playershipinfo_2) (Variables|AsteroidInfo|GetOre))))))))))))

(event EventBeginPlay)

(event Collision|EventActorBeginOverlap
  (params (OtherActor :type Actor%20Object%20Reference)))

(event EventTick
  (params (DeltaSeconds :type Float%20%28single-precision%29))
  ;[0 1 0.8125] Set Asteroid to auto-rotate
  (Transformation|AddLocalRotation (Variables|Default|GetRenderComponent) (* (Math|Rotator|MakeRotator 0.0 (Variables|Default|GetRotationSpeed) 0.0) DeltaSeconds) false false))

(fn ConstructionScript
  (bind _returnvalue (Math|Random|RandomFloatinRange 0.5 1.0))
  (bind _rendercomponent (Variables|Default|GetRenderComponent))
  (bind _sphere (Variables|Default|GetSphere))
  (bind _returnvalue_2 (Math|Vector|MakeVector _returnvalue _returnvalue _returnvalue))
  (Transformation|SetWorldRotation _rendercomponent (Math|Rotator|MakeRotator 0.0 (.pitch (Math|Random|RandomRotator false)) 0.0) false false)
  (Transformation|SetWorldScale3D _rendercomponent _returnvalue_2)
  (Transformation|SetWorldScale3D _sphere (+ (+ _returnvalue_2 1.0) (Transformation|GetWorldScale _sphere))) ; Slightly increase the scale of\nthe collision sphere according\nto the size of the asteroid
)

(fn ReferenceCasts
  (params (Object :type Object%20Object%20Reference))
  (bind _asbp_character (Utilities|Casting|CastToBP_Character Object))
  (bind _output_get (Variables|Default|SetPlayerCharRef _asbp_character))
  (bind _asbp_player_controller (Utilities|Casting|CastToBP_PlayerController (Pawn|GetController _output_get)))
  (Variables|Default|SetPlayerControllerRef _asbp_player_controller))