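; BPC_Attack is an attack component that lets enemies shoot at the player and handles killing the player.
; On BeginPlay it caches references to BP_GameMode and the player's BP_Character.
; ShootPlayer spawns a BP_Projectile at the enemy's flipbook, rotated toward the player's sprite; its line trace result is unused.
; DestroyPlayer shows the explosion flipbook, zeroes the controller's default movement speed and calls its death handler.
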(event EventBeginPlay
  (CallFunction|ReferenceCasts))

(event EventTick
  (params (DeltaSeconds :type Float%20%28single-precision%29)))

(fn DestroyPlayer
  (bind _playercharref (Variables|References|GetPlayerCharRef))
  ;[0.9922 0 1] Destroy Player
  (Rendering|SetVisibility (Variables|/Game/Blueprints/Player/BP_Character.BP_Character_C|GetExplodeFlipbook _playercharref) true true)
  (bind _asbp_player_controller (Utilities|Casting|CastToBP_PlayerController (Pawn|GetController _playercharref)))
  (Variables|References|SetPlayerControllerRef _asbp_player_controller)
  (Variables|/Game/Blueprints/Player/BP_PlayerController.BP_PlayerController_C|SetDefaultPlayerMovementSpeed (Variables|References|GetPlayerControllerRef) 0.0)
  (Default|HandlePlayerDeath (Variables|References|GetPlayerControllerRef)))

(fn ReferenceCasts
  (bind _asbp_game_mode (Utilities|Casting|CastToBP_GameMode (Game|GetGameMode)))
  (Variables|References|SetGameModeRef _asbp_game_mode)
  (bind _asbp_character (Utilities|Casting|CastToBP_Character (Game|GetPlayerCharacter 0)))
  (Variables|References|SetPlayerCharRef _asbp_character))

(fn ShootPlayer
  (params (Enemy :type BP%20Enemy%20Ship%20Object%20Reference))
  (bind _playercharref (Variables|References|GetPlayerCharRef))
  (bind _paperflipbook (Variables|/Game/Blueprints/Enemy/BP_EnemyBase.BP_EnemyBase_C|GetPaperFlipbook Enemy))
  (bind _returnvalue (Transformation|GetWorldLocation _paperflipbook))
  (bind _sprite (Variables|/Script/Paper2D.PaperCharacter|GetSprite _playercharref))
  (bind _returnvalue_2 (Transformation|GetWorldLocation _sprite))
  (Collision|LineTraceByChannel _returnvalue _returnvalue_2 "TraceTypeQuery1" false 0 "None")
  (bind _returnvalue_3 (Game|SpawnActorfromClass "/Game/Blueprints/BP_Projectile.BP_Projectile_C" (Math|Transform|MakeTransform _returnvalue (Math|Rotator|FindLookatRotation _returnvalue _returnvalue_2) "1,1,1") "Undefined" 0 0))
  (Variables|References|SetProjectileRef _returnvalue_3))