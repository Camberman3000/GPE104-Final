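; BP_EnemyShip is a patrolling enemy ship that attacks the player on detection.
; A timeline lerps its flipbook toward EndLocation at a rate set by travel time, loitering before replaying.
; DangerSphere overlap with BP_Character stops the patrol, then fires BPCAttack's shoot and delayed destroy, with BPCSounds audio.
; The construction script previews the end location and copies ScanRange into BP_GameMode for difficulty.
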(event OnComponentBeginOverlap(DangerSphere)
  (params (OverlappedComponent :type Primitive%20Component%20Object%20Reference) (OtherActor :type Actor%20Object%20Reference) (OtherComp :type Primitive%20Component%20Object%20Reference) (OtherBodyIndex :type Integer) (bFromSweep :type Boolean) (SweepResult :type Hit%20Result%20Structure%20%28by%20ref%29))
  (bind _bpc_attack (Variables|Default|GetBPC_Attack))
  ;[0 0.7422 1] Enemy Overlap
  (bind _asbp_character (Utilities|Casting|CastToBP_Character OtherActor))
  (Variables|References|SetPlayerCharRef _asbp_character)
  (Default|PlaySound (Variables|Default|GetBPC_Sounds) "/Game/Retro_8Bit_Sounds/Teleport/Wavs/retro_teleport_warp_effect_39.retro_teleport_warp_effect_39" 1.0) ; Tractor beam
  (Utilities|FlowControl|Delay 0.2)
  (CallFunction|StopPatrol)
  (Default|ShootPlayer _bpc_attack self)
  (Utilities|FlowControl|Delay 1.0)
  (Default|DestroyPlayer _bpc_attack)
  (Default|PlaySound (Variables|Default|GetBPC_Sounds) "/Game/Retro_8Bit_Sounds/Explosion/Wavs/retro_explosion_general_01.retro_explosion_general_01" 1.0))

(event Custom|PlayFromStart
  ;[1 0.2812 0] Patrol
  (bind _lerp_alpha (Timeline|PatrolTimeline PlayFromStart)
    (:Update
      (Transformation|SetRelativeLocation (Variables|Default|GetPaperFlipbook) (Math|Vector|Lerp(Vector) "0,100.000000, 0" (Variables|PatrolInfo|GetEndLocation) _lerp_alpha) false false))
    (:Finished
      (Utilities|FlowControl|Delay (Variables|PatrolInfo|GetLoiterTime))
      (CallFunction|PlayfromStart))))

(event Custom|PlayBackward
  ;[1 0.2812 0] Patrol
  (bind _lerp_alpha (Timeline|PatrolTimeline ReverseFromEnd)
    (:Update
      (Transformation|SetRelativeLocation (Variables|Default|GetPaperFlipbook) (Math|Vector|Lerp(Vector) "0,100.000000, 0" (Variables|PatrolInfo|GetEndLocation) _lerp_alpha) false false))
    (:Finished
      (Utilities|FlowControl|Delay (Variables|PatrolInfo|GetLoiterTime))
      (CallFunction|PlayfromStart))))

(event Custom|StopPatrol
  ;[1 0.2812 0] Patrol
  (bind _lerp_alpha (Timeline|PatrolTimeline Stop)
    (:Update
      (Transformation|SetRelativeLocation (Variables|Default|GetPaperFlipbook) (Math|Vector|Lerp(Vector) "0,100.000000, 0" (Variables|PatrolInfo|GetEndLocation) _lerp_alpha) false false))
    (:Finished
      (Utilities|FlowControl|Delay (Variables|PatrolInfo|GetLoiterTime))
      (CallFunction|PlayfromStart))))

(event Custom|PlayPatrol
  ;[1 0.2812 0] Patrol
  (bind _lerp_alpha (Timeline|PatrolTimeline Play)
    (:Update
      (Transformation|SetRelativeLocation (Variables|Default|GetPaperFlipbook) (Math|Vector|Lerp(Vector) "0,100.000000, 0" (Variables|PatrolInfo|GetEndLocation) _lerp_alpha) false false))
    (:Finished
      (Utilities|FlowControl|Delay (Variables|PatrolInfo|GetLoiterTime))
      (CallFunction|PlayfromStart))))

(event EventBeginPlay
  (|CallParentFunction)
  (Components|Timeline|SetPlayRate (Variables|Default|GetPatrolTimeline) (/ 1.0 (Variables|PatrolInfo|GetTravelTimeInSecconds)))
  (Variables|PatrolInfo|SetTestEndLocation? false))

(event Collision|EventActorBeginOverlap
  (params (OtherActor :type Actor%20Object%20Reference))
  (|CallParentFunction OtherActor) ; This node is disabled and will not be called.\nDrag off pins to build functionality.
)

(event EventTick
  (params (DeltaSeconds :type Float%20%28single-precision%29))
  (|CallParentFunction DeltaSeconds))

(fn ConstructionScript
  (|CallParentFunction)
  ;[0 1 0.1562] Test End Location
  (Transformation|SetRelativeLocation (Variables|Default|GetPaperFlipbook) (Math|Vector|SelectVector (Variables|PatrolInfo|GetEndLocation) "0,100.000000, 0" (Variables|PatrolInfo|GetTestEndLocation?)) false false)
  ;[0.1953 0 1] Set scan range var in game mode for
  ; difficulty setting
  (bind _asbp_game_mode (Utilities|Casting|CastToBP_GameMode (Game|GetGameMode)))
  (Variables|/Game/Blueprints/Game/BP_GameMode.BP_GameMode_C|SetScanRange _asbp_game_mode (Variables|Default|GetScanRange)))